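; Player character Blueprint that links a main menu widget to grapple-based play and restarts the level when the player falls.
; BeginPlay enables touch joysticks and the mouse cursor, then creates the menu widget if needed.
; StartGame blocks walking off ledges and activates the grapple component, while OpenMainMenu shows the menu and deactivates it.
; Tick detects dropping below a height threshold, triggering a one-shot game-over display and delayed reload of the current level.
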(event `self.ReceiveBeginPlay`
  (bind _returnvalue (`self.GetLocalViewingPlayerController`))
  (`PlayerController.ActivateTouchInterface` _returnvalue "/Engine/MobileResources/HUD/DefaultVirtualJoysticks.DefaultVirtualJoysticks")
  (set `PlayerController.bShowMouseCursor` true _returnvalue)
  (`self.WBP Main Menu`
    (:`then`
      _)
    (:`else`
      (bind _returnvalue_2 (`|CreateWidget` "/Game/Assignment/Blueprints/Widgets/WBP_MainMenu.WBP_MainMenu_C" _returnvalue))
      (bind _output_get (set `self.WBP Main Menu` _returnvalue_2))
      (`UserWidget.AddToViewport` _output_get 0)))
  (`/Game/Assignment/Blueprints/Widgets/WBP_MainMenu.ResetGameOver` _output_get))

(event `StartGame`
  ;[0.02029 0.02029 0.02029] Ensure Player cannot walk off ledges
  (set `CharacterMovementComponent.bCanWalkOffLedges` false (`self.CharacterMovement`))
  (`ActorComponent.Activate` (`self.GrappleComponent`) false))

(event `self.ReceiveTick`
  (params (DeltaSeconds :type "Float (single-precision)"))
  (bind (_returnvalue_x _returnvalue_y _returnvalue_z) (`KismetMathLibrary.BreakVector` (`self.K2_GetActorLocation`)))
  (bind _wbp_main_menu (`self.WBP Main Menu`))
  ;[0.05 0.05 0.05] Reset Level if Player falls off
  (if (or (and (`NavMovementComponent.IsFalling` (`self.CharacterMovement`)) (< _returnvalue_z -1.0)) (< _returnvalue_z -1.0))
    (`/Engine/EditorBlueprintResources/StandardMacros.DoOnce` false :!label _label
      (:`Completed`
        (`Widget.SetVisibility` _wbp_main_menu "Visible")
        (`/Game/Assignment/Blueprints/Widgets/WBP_MainMenu.GameOverEvent` _wbp_main_menu)
        (`KismetSystemLibrary.Delay` 2.0)
        (`self.Respawn`)))))

(event `Respawn`
  ;[0.05 0.05 0.05] Reset Level if Player falls off
  (`/Game/Assignment/Blueprints/Widgets/WBP_MainMenu.ResetGameOver` (`self.WBP Main Menu`))
  (bind _returnvalue (`GameplayStatics.GetCurrentLevelName` true))
  (`GameplayStatics.OpenLevel` (`KismetStringLibrary.Conv_StringToName` _returnvalue))
  (goto _label :!via `Reset`))

(event `OpenMainMenu`
  (`Widget.SetVisibility` (`self.WBP Main Menu`) "Visible")
  (`ActorComponent.Deactivate` (`self.GrappleComponent`)))

(fn `UserConstructionScript`
  (`parent.UserConstructionScript`))