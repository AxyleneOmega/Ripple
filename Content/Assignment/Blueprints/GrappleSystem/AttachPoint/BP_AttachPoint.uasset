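; BP_AttachPoint is a grapple system attach point actor that shows a hover indicator through a widget component.
; On BeginPlay it casts the component's widget to WBP_AttachPoint and caches it.
; Activate stores the instigating pawn, sets the active flag and turns on the widget's hover state, while Deactivate reverses all three.
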(event `self.ReceiveBeginPlay`
  (bind _aswbp_attach_point (cast `/Game/Assignment/Blueprints/GrappleSystem/AttachPoint/WBP_AttachPoint` (`WidgetComponent.GetWidget` (`self.Widget`))))
  (set `self.Widget Attach Point` _aswbp_attach_point))

(event `/Game/Assignment/Blueprints/Interfaces/I_Interact.Activate`
  (params (`Instigating Pawn` :type "/Game/Assignment/Blueprints/BP_PlayerChar Object Reference"))
  (set `self.Instigating Pawn` `Instigating Pawn`)
  (bind _output_get (set `self.isActive?` true))
  (`/Game/Assignment/Blueprints/GrappleSystem/AttachPoint/WBP_AttachPoint.Hovering?` (`self.Widget Attach Point`) _output_get))

(event `/Game/Assignment/Blueprints/Interfaces/I_Interact.Deactivate`
  (bind _output_get (set `self.isActive?` false))
  (`/Game/Assignment/Blueprints/GrappleSystem/AttachPoint/WBP_AttachPoint.Hovering?` (`self.Widget Attach Point`) _output_get)
  (set `self.Instigating Pawn` null))

(fn `UserConstructionScript`)