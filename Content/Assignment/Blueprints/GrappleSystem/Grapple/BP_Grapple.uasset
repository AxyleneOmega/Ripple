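; Grapple hook projectile that flies along a set direction and expires after a few seconds unless it reaches its impact point.
; Each tick a small sphere overlap at the precomputed impact point checks for the hook itself, rather than relying on collision hits.
; On arrival it stops, snaps to the point, clears its lifespan, reports success and plays a click pitched by whether an attach point reference is valid.
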(event `self.ReceiveBeginPlay`
  (set `MovementComponent.Velocity` (* (`self.Direction`) (`self.ShootSpeed`)) (`self.ProjectileMovement`))
  (`self.SetLifeSpan` 5.0))

(event `self.ReceiveTick`
  (params (DeltaSeconds :type "Float (single-precision)"))
  (bind _impactpoint (`self.ImpactPoint`))
  (bind (_outactors _returnvalue) (`KismetSystemLibrary.SphereOverlapActors` _impactpoint 32.0 (`|MakeArray` "ObjectTypeQuery2" :!type "EObjectTypeQuery Enum") "BP_Grapple_C"))
  (if (and _returnvalue (`KismetArrayLibrary.Array_Contains` _outactors self))
    (`/Engine/EditorBlueprintResources/StandardMacros.DoOnce` false :!label _label
      (:`Completed`
        (set `MovementComponent.Velocity` (0.0 0.0 0.0) (`self.ProjectileMovement`))
        (`self.K2_SetActorLocation` _impactpoint)
        (`self.SetLifeSpan` 0.0)
        (`self.GrappleResult` true)
        (`self.AttachPointRef`
          (:`then`
            (set `self.ClickPitch` 0.6))
          (:`else`
            (set `self.ClickPitch` 1.3)))
        (`GameplayStatics.PlaySoundAtLocation` "/Game/Assignment/Assets/Sounds/mixkit-hard-click-1118.mixkit-hard-click-1118" _impactpoint (struct) 0.5 (`self.ClickPitch`) 0.1 null null self null)))
    (else
      (goto _label :!via `Reset`))))

(fn `GetAttachPointLocation`
  (returns (ReturnValue :type "Vector Structure"))
  (return (`KismetMathLibrary.TransformLocation` (`self.GetTransform`) (`self.ImpactPoint`))))

(fn `UserConstructionScript`)